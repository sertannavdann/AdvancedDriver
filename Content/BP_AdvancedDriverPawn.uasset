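; BP_AdvancedDriverPawn is a driver pawn that exposes vehicle speed and gear values, likely for a UMG dashboard.
; BeginPlay assigns UMG_Panel to DriverWidgetClass.
; Each Tick parses SpeedDisplayString into an integer Speed, derives SpeedNormalized on a hundred-unit scale without clamping, and copies GearDisplayString into Gear.
; Speed comes from display text rather than a numeric movement value, and the construction script is empty.
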(event EventTick
  (params (DeltaSeconds :type Float%20%28single-precision%29))
  (bind _speeddisplaystring (Variables|Default|GetSpeedDisplayString))
  (bind _returnvalue (Utilities|String|ToString(Text) _speeddisplaystring))
  (bind _returnvalue_2 (Math|Conversions|ToInteger(Byte) _returnvalue))
  (switch int _returnvalue_2
    (:Default
      (bind _output_get (Variables|HUD|SetSpeed _returnvalue_2))
      (Variables|HUD|SetSpeedNormalized (/ (Math|Conversions|ToFloat(Integer) _output_get) 1e+02))
      (Variables|HUD|SetGear (Variables|Default|GetGearDisplayString)))))

(event EventBeginPlay
  (Variables|Default|SetDriverWidgetClass "/Game/UMG_Panel.UMG_Panel_C"))

(fn ConstructionScript)